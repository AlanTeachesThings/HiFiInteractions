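; Base interactive object that registers itself with the third-person character while inside its activation collider, with an empty Interact event.
; Leaving the collider unregisters it and removes the highlight.
; SetNearestObjectToPlayer uses two DoOnce gates that reset each other, so highlight and de-highlight each fire only once per change in nearest status.
; The highlight actions only toggle a debug billboard's visibility, when debugging is enabled.
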(event OnComponentBeginOverlap(ActivationCollider)
  (params (OverlappedComponent :type Primitive%20Component%20Object%20Reference) (OtherActor :type Actor%20Object%20Reference) (OtherComp :type Primitive%20Component%20Object%20Reference) (OtherBodyIndex :type Integer) (bFromSweep :type Boolean) (SweepResult :type Hit%20Result%20Structure%20%28by%20ref%29))
  (bind _asbp_third_person_character (Utilities|Casting|CastToBP_ThirdPersonCharacter OtherActor))
  (Default|AddInteractableObject _asbp_third_person_character self))

(event OnComponentEndOverlap(ActivationCollider)
  (params (OverlappedComponent :type Primitive%20Component%20Object%20Reference) (OtherActor :type Actor%20Object%20Reference) (OtherComp :type Primitive%20Component%20Object%20Reference) (OtherBodyIndex :type Integer))
  (bind _asbp_third_person_character (Utilities|Casting|CastToBP_ThirdPersonCharacter OtherActor))
  (Default|RemoveInteractiveObject _asbp_third_person_character self)
  (CallFunction|DeHighlightActions))

(event Custom|Interact
  (params (InstigatingCharacter :type BP%20Third%20Person%20Character%20Object%20Reference)))

(event EventBeginPlay)

(event Collision|EventActorBeginOverlap
  (params (OtherActor :type Actor%20Object%20Reference)))

(event EventTick
  (params (DeltaSeconds :type Float%20%28single-precision%29)))

(fn ConstructionScript)

(fn SetNearestObjecttoPlayer
  (params (isNearestObject :type Boolean))
  (bind _output_get (Variables|Default|SetisNearestObject isNearestObject))
  (if _output_get
    ;[1 1 1] Only ever trigger Highlight/DeHighlight Once - then reset the opposite
    (Utilities|FlowControl|DoOnce false :!label _label
      (:Completed
        (CallFunction|HighlightActions)
        (goto _label_2 Reset)))
    (else
      (Utilities|FlowControl|DoOnce false :!label _label_2
        (:Completed
          (CallFunction|DeHighlightActions)
          (goto _label Reset))))))

(fn HighlightActions
  (if (Variables|Default|GetdebugHighlightActions)
    (Rendering|SetVisibility (Variables|Default|GetDebugBillboard) true false)))

(fn DeHighlightActions
  (if (Variables|Default|GetdebugHighlightActions)
    (Rendering|SetVisibility (Variables|Default|GetDebugBillboard) false false)))